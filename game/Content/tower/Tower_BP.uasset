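; Tower actor for a tower-defense style game that automatically fires projectiles at AI_RUNNER targets, configured by TowerStruct.
; Targets come from range-sphere overlaps or a Tick-called sphere trace that picks the closest runner, and clear on leaving range.
; Tick fires homing-target projectiles carrying damage, gated by a fire-rate reload delay.
; The scan's throttle flag is only ever set false, so it never blocks rescans.
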(event `check_for_new_target`
  (bind _returnvalue (`self.K2_GetActorLocation`))
  (set `self.Check_For_Target_Delay` false)
  (bind (_outhits _returnvalue_2) (`KismetSystemLibrary.SphereTraceMultiForObjects` _returnvalue (- _returnvalue (0.0 0.0 1.0)) (`.Range_7_77FD88054058FCBCECEBAC951A4587FF` (break `/Game/tower/Tower_Structure` (`self.TowerStruct`))) (`|MakeArray` "ObjectTypeQuery3" :!type "EObjectTypeQuery Enum")))
  (if _returnvalue_2
    (bind _newparam (`self.Closet Target Calculation` _outhits))
    (`/Engine/EditorBlueprintResources/StandardMacros.IsValid` _newparam
      (:`Is Valid`
        (set `self.Tower_Target` _newparam))
      (:`Is Not Valid`
        _)))
  (`KismetSystemLibrary.Delay` 0.2)
  (set `self.Check_For_Target_Delay` false))

(event `self.ReceiveTick`
  (params (DeltaSeconds :type "Float (single-precision)"))
  (`/Engine/EditorBlueprintResources/StandardMacros.IsValid` (`self.Tower_Target`)
    (:`Is Valid`
      (if (not (`self.Reload`))
        (`self.Shoot`)))
    (:`Is Not Valid`
      (if (not (`self.Check_For_Target_Delay`))
        (`self.check_for_new_target`)))))

(event `Shoot`
  (bind (_name _damage _range _fire_rate) (break `/Game/tower/Tower_Structure` (`self.TowerStruct`)))
  (set `self.Reload` true)
  (`|SpawnActorFromClass` "/Game/tower/Projectile.Projectile_C" (`self.GetTransform`) "AlwaysSpawn" "OverrideRootScale" null (`self.Tower_Target`) _damage null)
  (`KismetSystemLibrary.Delay` _fire_rate)
  (set `self.Reload` false))

(event `Tower_Instance`
  (bind (_name _damage _range _fire_rate _mesh) (break `/Game/tower/Tower_Structure` (`self.TowerStruct`)))
  (`StaticMeshComponent.SetStaticMesh` (`self.Tower`) _mesh)
  (`SphereComponent.SetSphereRadius` (`self.Sphere`) _range true))

(event `self.Sphere.OnComponentBeginOverlap`
  (params (OverlappedComponent :type "PrimitiveComponent Object Reference") (OtherActor :type "Actor Object Reference") (OtherComp :type "PrimitiveComponent Object Reference") (OtherBodyIndex :type Integer) (bFromSweep :type Boolean) (SweepResult :type "HitResult Structure (by ref)"))
  (`/Engine/EditorBlueprintResources/StandardMacros.IsValid` (`self.Tower_Target`)
    (:`Is Not Valid`
      (bind _asai_runner (cast `/Game/AI/AI_RUNNER` OtherActor))
      (set `self.Tower_Target` _asai_runner))))

(event `self.Sphere.OnComponentEndOverlap`
  (params (OverlappedComponent :type "PrimitiveComponent Object Reference") (OtherActor :type "Actor Object Reference") (OtherComp :type "PrimitiveComponent Object Reference") (OtherBodyIndex :type Integer))
  (if (== (`self.Tower_Target`) OtherActor)
    (set `self.Tower_Target` null)))

(event `self.ReceiveBeginPlay`)

(fn `Closet Target Calculation`
  (params (Hit_Result :type "Array of HitResult Structure"))
  (returns (NewParam :type "/Game/AI/AI_RUNNER Object Reference"))
  (locals (Temp_Target :type "/Game/AI/AI_RUNNER Object Reference") (Temp_Distance :type "Float (double-precision)" :default 0.0))
  (for _array_element Hit_Result
    (bind (_bblockinghit _binitialoverlap _time _distance _location _impactpoint _normal _impactnormal _physmat _hitactor) (`GameplayStatics.BreakHitResult` _array_element))
    (bind _asai_runner (cast `/Game/AI/AI_RUNNER` _hitactor))
    (`/Engine/EditorBlueprintResources/StandardMacros.IsValid` (`local.Temp_Target`)
      (:`Is Valid`
        (bind _returnvalue (`KismetMathLibrary.VSize` (- (`self.K2_GetActorLocation`) (`self.K2_GetActorLocation` _hitactor))))
        (if (< _returnvalue (`local.Temp_Distance`))
          (set `local.Temp_Target` _asai_runner)
          (set `local.Temp_Distance` _returnvalue)))
      (:`Is Not Valid`
        (set `local.Temp_Target` _asai_runner)
        (set `local.Temp_Distance` _returnvalue))))
  (return (`local.Temp_Target`)))

(fn `UserConstructionScript`)
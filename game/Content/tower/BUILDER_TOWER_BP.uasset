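; BUILDER_TOWER_BP is the placement ghost that previews where a tower can be built.
; Each Tick it snaps the cursor's world hit to an XY grid and line-traces down onto that point, moving there when an actor is hit.
; A "Wall" tag on that actor enables building and turns the ghost green, otherwise red.
; Place_Tower, when building is allowed, spawns Tower_BP with TowerData, calls TowerInstance and destroys the ghost.
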(event `self.ReceiveTick`
  (params (DeltaSeconds :type "Float (single-precision)"))
  (bind _ghost_tower (`self.Ghost_Tower`))
  (bind (_hitresult _returnvalue) (`PlayerController.GetHitResultUnderCursorForObjects` (`GameplayStatics.GetPlayerController` 0) (`|MakeArray` "ObjectTypeQuery1" :!type "EObjectTypeQuery Enum") true))
  (bind _returnvalue_2 (`PrimitiveComponent.GetMaterial` _ghost_tower 0))
  ;[1 1 1] tower placement and snapping
  (if _returnvalue
    (bind _output_get (set `self.Snap_Location` (`KismetMathLibrary.MakeVector` (`KismetMathLibrary.GridSnap_Float` (.x (`.Location` (`GameplayStatics.BreakHitResult` _hitresult))) 50.0) (`KismetMathLibrary.GridSnap_Float` (.y (`.Location` (`GameplayStatics.BreakHitResult` _hitresult))) 50.0) (.z (`.Location` (`GameplayStatics.BreakHitResult` _hitresult))))))
    (bind _outhit (`KismetSystemLibrary.LineTraceSingleForObjects` :`Start` (+ _output_get (0.0 0.0 50.0)) :`End` _output_get :`ObjectTypes` (`|MakeArray` "ObjectTypeQuery1" :!type "EObjectTypeQuery Enum") :`DrawDebugType` "ForDuration"))
    (bind (_bblockinghit _binitialoverlap _time _distance _location _impactpoint _normal _impactnormal _physmat _hitactor) (`GameplayStatics.BreakHitResult` _outhit))
    (`/Engine/EditorBlueprintResources/StandardMacros.IsValid` _hitactor
      (:`Is Valid`
        (if (`self.ActorHasTag` _hitactor "Wall")
          (set `self.Can_Build` true)
          (if (not (== _returnvalue_2 "/Game/tower/GREEN_TRANSLUCENT.GREEN_TRANSLUCENT"))
            (`PrimitiveComponent.SetMaterial` _ghost_tower 0 "/Game/tower/GREEN_TRANSLUCENT.GREEN_TRANSLUCENT")
            (`KismetSystemLibrary.PrintString` "turn green"))
          (else
            (set `self.Can_Build` false)
            (if (not (== _returnvalue_2 "/Game/tower/RED_TRANSLUCENT1.RED_TRANSLUCENT1"))
              (`PrimitiveComponent.SetMaterial` _ghost_tower 0 "/Game/tower/RED_TRANSLUCENT1.RED_TRANSLUCENT1")
              (`KismetSystemLibrary.PrintString` "turn red"))))
        (`self.K2_SetActorLocation` (`self.Snap_Location`))))))

(event `Place_Tower`
  ;[1 1 1] Place Tower
  (if (`self.Can_Build`)
    (bind _returnvalue (`|SpawnActorFromClass` "/Game/tower/Tower_BP.Tower_BP_C" (`self.GetTransform`) "Undefined" "OverrideRootScale" null null))
    (set `/Game/tower/Tower_BP.TowerStruct` (`self.Tower_Data`) _returnvalue)
    (`/Game/tower/Tower_BP.Tower_Instance` _returnvalue)
    (`self.K2_DestroyActor`)))

(fn `UserConstructionScript`)